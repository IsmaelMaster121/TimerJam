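; Main menu player that shows the mouse cursor and moves the camera between Play, Credits, Config, Sound and Graphics views.
; Tick reads nested bool flags to play or reverse a timeline per view, lerping the camera's relative transform, with Sound and Graphics offsets added onto the Config move.
; The Play move also carries a Box, whose overlap with BP_AutoMuestra swaps chassis and grille materials after a delay to light the car.
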(event OnComponentBeginOverlap(Box)
  (params (OverlappedComponent :type Primitive%20Component%20Object%20Reference) (OtherActor :type Actor%20Object%20Reference) (OtherComp :type Primitive%20Component%20Object%20Reference) (OtherBodyIndex :type Integer) (bFromSweep :type Boolean) (SweepResult :type Hit%20Result%20Structure%20%28by%20ref%29))
  ;[0 0.5245 1] Prende las Luces
  (Utilities|FlowControl|Delay 0.8)
  (bind _asbp_auto_muestra (Utilities|Casting|CastToBP_AutoMuestra OtherActor))
  (Actor|GetActorOfClass "/Game/VehicleTemplate/Blueprints/OffroadCar/BP_AutoMuestra.BP_AutoMuestra_C")
  ;;[1 0 0] Chasis
  (Rendering|Material|SetMaterial (Variables|/Script/TimerJamProyect.TimerJamProyectOffroadCar|GetChassis _asbp_auto_muestra) 4 "/Game/Vehicles/OffroadCar/CarMaterials/LuzBlanca3.LuzBlanca3")
  (Rendering|Material|SetMaterial (Variables|/Script/TimerJamProyect.TimerJamProyectOffroadCar|GetChassis _asbp_auto_muestra) 11 "/Game/Vehicles/OffroadCar/CarMaterials/LuzBlanca3.LuzBlanca3")
  (Rendering|Material|SetMaterial (Variables|/Script/TimerJamProyect.TimerJamProyectOffroadCar|GetChassis _asbp_auto_muestra) 12 "/Game/Vehicles/OffroadCar/CarMaterials/LuzNaranja3.LuzNaranja3")
  (Rendering|Material|SetMaterial (Variables|/Script/TimerJamProyect.TimerJamProyectOffroadCar|GetChassis _asbp_auto_muestra) 12 "/Game/Vehicles/OffroadCar/CarMaterials/LuzNaranja3.LuzNaranja3")
  ;;[0.9978 0.1834 1] parrilla
  (Rendering|Material|SetMaterial (Variables|/Game/VehicleTemplate/Blueprints/OffroadCar/BP_AutoMuestra.BP_AutoMuestra_C|Getparrila _asbp_auto_muestra) 1 "/Game/Vehicles/OffroadCar/CarMaterials/LuzBlanca.LuzBlanca")
  (Rendering|Material|SetMaterial (Variables|/Game/VehicleTemplate/Blueprints/OffroadCar/BP_AutoMuestra.BP_AutoMuestra_C|Getparrila _asbp_auto_muestra) 2 "/Game/Vehicles/OffroadCar/CarMaterials/LuzBlanca.LuzBlanca")
  (Rendering|Material|SetMaterial (Variables|/Game/VehicleTemplate/Blueprints/OffroadCar/BP_AutoMuestra.BP_AutoMuestra_C|Getparrila _asbp_auto_muestra) 4 "/Game/Vehicles/OffroadCar/CarMaterials/LuzBlanca.LuzBlanca")
  (Rendering|Material|SetMaterial (Variables|/Game/VehicleTemplate/Blueprints/OffroadCar/BP_AutoMuestra.BP_AutoMuestra_C|Getparrila _asbp_auto_muestra) 6 "/Game/Vehicles/OffroadCar/CarMaterials/LuzBlanca.LuzBlanca")
  (Rendering|Material|SetMaterial (Variables|/Game/VehicleTemplate/Blueprints/OffroadCar/BP_AutoMuestra.BP_AutoMuestra_C|Getparrila _asbp_auto_muestra) 8 "/Game/Vehicles/OffroadCar/CarMaterials/LuzBlanca.LuzBlanca"))

(event EventBeginPlay
  ;[1 0.6144 0.9459] Para que no se oculte el mouse
  (Variables|/Script/Engine.PlayerController|SetbShowMouseCursor (Game|GetPlayerController 0) true))

(event EventTick
  (params (DeltaSeconds :type Float%20%28single-precision%29))
  (if (Variables|Default|GetShould)
    (if (Variables|Default|GetShould2)
      (if (Variables|Default|GetShould3)
        (if (Variables|Default|GetShould4)
          ;[1 0 0] Cambio Graficos
          (if (Variables|Default|GetGraficosACT)
            (bind _movimientosecsi (Timeline|Timeline_Grafics Play)
              (:Update
                (Transformation|SetRelativeLocationAndRotation (Variables|Default|GetCamera) (Math|Vector|MakeVector (+ (Math|Float|Lerp 0.0 -5.5e+02 _movimientosecsi) (Math|Float|Lerp 0.0 3.5e+03 (stale _movimientosecsi_3))) (+ (Math|Float|Lerp 0.0 -4.5e+02 _movimientosecsi) (Math|Float|Lerp 0.0 -3.5e+02 (stale _movimientosecsi_3))) (+ (Math|Float|Lerp 0.0 0.0 _movimientosecsi) (Math|Float|Lerp 0.0 -3e+02 (stale _movimientosecsi_3)))) (Math|Rotator|MakeRotator 0.0 (Math|Float|Lerp 0.0 -8e+01 (stale _movimientosecsi_3)) (Math|Float|Lerp 0.0 -49.0 (stale _movimientosecsi_3))) false false)))
            (else
              (Timeline|Timeline_Grafics Reverse)))
          (else
            ;[0 1 0.1192] Cambio Sonido
            (if (Variables|Default|GetSoundACT)
              (bind _movimientosecsi_2 (Timeline|Timeline_1 Play)
                (:Update
                  (Transformation|SetRelativeLocationAndRotation (Variables|Default|GetCamera) (Math|Vector|MakeVector (+ (Math|Float|Lerp 0.0 3.5e+03 (stale _movimientosecsi_3)) (Math|Float|Lerp 0.0 5.5e+02 _movimientosecsi_2)) (+ (Math|Float|Lerp 0.0 -3.5e+02 (stale _movimientosecsi_3)) (Math|Float|Lerp 0.0 4.5e+02 _movimientosecsi_2)) (+ (Math|Float|Lerp 0.0 -3e+02 (stale _movimientosecsi_3)) (Math|Float|Lerp 0.0 0.0 _movimientosecsi_2))) (Math|Rotator|MakeRotator 0.0 (Math|Float|Lerp 0.0 -8e+01 (stale _movimientosecsi_3)) (Math|Float|Lerp 0.0 -49.0 (stale _movimientosecsi_3))) false false)))
              (else
                (Timeline|Timeline_1 Reverse)))))
        (else
          ;[0 0.01226 1] Cambio Config
          (if (Variables|Default|GetConfigACT)
            (bind _movimientosecsi_3 (Timeline|Timeline Play)
              (:Update
                (Transformation|SetRelativeLocationAndRotation (Variables|Default|GetCamera) (Math|Vector|MakeVector (Math|Float|Lerp 0.0 3.5e+03 _movimientosecsi_3) (Math|Float|Lerp 0.0 -3.5e+02 _movimientosecsi_3) (Math|Float|Lerp 0.0 -3e+02 _movimientosecsi_3)) (Math|Rotator|MakeRotator 0.0 (Math|Float|Lerp 0.0 -8e+01 _movimientosecsi_3) (Math|Float|Lerp 0.0 -49.0 _movimientosecsi_3)) false false)))
            (else
              (Timeline|Timeline Reverse)))))
      (else
        ;[1 0.8743 0] Cambio Creditos
        (if (Variables|Default|GetCreditsAct)
          (bind _movimientosecsi_4 (Timeline|Mov Play)
            (:Update
              (Transformation|SetRelativeLocationAndRotation (Variables|Default|GetCamera) (Math|Vector|MakeVector (Math|Float|Lerp 0.0 1.6e+03 _movimientosecsi_4) (Math|Float|Lerp 0.0 -1.2e+03 _movimientosecsi_4) (Math|Float|Lerp 0.0 -4e+02 _movimientosecsi_4)) (Math|Rotator|MakeRotator 0.0 (Math|Float|Lerp 0.0 -1e+01 _movimientosecsi_4) (Math|Float|Lerp 0.0 -7e+01 _movimientosecsi_4)) false false)))
          (else
            (Timeline|Mov Reverse)))))
    (else
      ;[0 0.8385 1] Cambio Play
      (if (Variables|Default|GetPlayACT)
        (bind _movimientosecsi_5 (Timeline|Mov2 Play)
          (:Update
            (Transformation|SetRelativeLocationAndRotation (Variables|Default|GetCamera) (Math|Vector|MakeVector (Math|Float|Lerp 0.0 1.8e+03 _movimientosecsi_5) (Math|Float|Lerp 0.0 5e+01 _movimientosecsi_5) (Math|Float|Lerp 0.0 -5e+02 _movimientosecsi_5)) (Math|Rotator|MakeRotator 0.0 (Math|Float|Lerp 0.0 0.0 _movimientosecsi_5) (Math|Float|Lerp 0.0 4e+01 _movimientosecsi_5)) false false)))
        (else
          (Timeline|Mov2 Reverse))))))

(fn ConstructionScript)