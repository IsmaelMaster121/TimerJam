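; BP_ToLevel2 is a trigger actor that repaints the offroad car and closes off invisible walls, apparently at the transition to Level 2.
; When BP_OffroadCar_Pawn enters BoxDetectora, it swaps materials slot by slot on the chassis, suitcase, wheels and grille.
; It then unhides Pared and enables its collision, doing the same for Pared1 after a short delay.
; Any end overlap on the box plays a 2D spray sound, with no actor check.
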(event OnComponentBeginOverlap(BoxDetectora)
  (params (OverlappedComponent :type Primitive%20Component%20Object%20Reference) (OtherActor :type Actor%20Object%20Reference) (OtherComp :type Primitive%20Component%20Object%20Reference) (OtherBodyIndex :type Integer) (bFromSweep :type Boolean) (SweepResult :type Hit%20Result%20Structure%20%28by%20ref%29))
  (bind _asbp_offroad_car_pawn (Utilities|Casting|CastToBP_OffroadCar_Pawn OtherActor))
  (Actor|GetActorOfClass "/Game/VehicleTemplate/Blueprints/OffroadCar/BP_OffroadCar_Pawn.BP_OffroadCar_Pawn_C")
  ;[1 0 0] Chasis
  (Rendering|Material|SetMaterial (Variables|/Script/TimerJamProyect.TimerJamProyectOffroadCar|GetChassis _asbp_offroad_car_pawn) 0 "/Game/Vehicles/OffroadCar/CarMaterials/Pintura2.Pintura2")
  (Rendering|Material|SetMaterial (Variables|/Script/TimerJamProyect.TimerJamProyectOffroadCar|GetChassis _asbp_offroad_car_pawn) 2 "/Game/Vehicles/OffroadCar/CarMaterials/Cromado2.Cromado2")
  (Rendering|Material|SetMaterial (Variables|/Script/TimerJamProyect.TimerJamProyectOffroadCar|GetChassis _asbp_offroad_car_pawn) 3 "/Game/Vehicles/OffroadCar/CarMaterials/Plastico2.Plastico2")
  (Rendering|Material|SetMaterial (Variables|/Script/TimerJamProyect.TimerJamProyectOffroadCar|GetChassis _asbp_offroad_car_pawn) 4 "/Game/Vehicles/OffroadCar/CarMaterials/LuzBlanca2.LuzBlanca2")
  (Rendering|Material|SetMaterial (Variables|/Script/TimerJamProyect.TimerJamProyectOffroadCar|GetChassis _asbp_offroad_car_pawn) 6 "/Game/Vehicles/OffroadCar/CarMaterials/Vidrio2.Vidrio2")
  (Rendering|Material|SetMaterial (Variables|/Script/TimerJamProyect.TimerJamProyectOffroadCar|GetChassis _asbp_offroad_car_pawn) 8 "/Game/Vehicles/OffroadCar/CarMaterials/CueroAsientos2.CueroAsientos2")
  (Rendering|Material|SetMaterial (Variables|/Script/TimerJamProyect.TimerJamProyectOffroadCar|GetChassis _asbp_offroad_car_pawn) 9 "/Game/Vehicles/OffroadCar/CarMaterials/Matricula2.Matricula2")
  (Rendering|Material|SetMaterial (Variables|/Script/TimerJamProyect.TimerJamProyectOffroadCar|GetChassis _asbp_offroad_car_pawn) 10 "/Game/Vehicles/OffroadCar/CarMaterials/LuzRoja2.LuzRoja2")
  (Rendering|Material|SetMaterial (Variables|/Script/TimerJamProyect.TimerJamProyectOffroadCar|GetChassis _asbp_offroad_car_pawn) 11 "/Game/Vehicles/OffroadCar/CarMaterials/LuzBlanca2.LuzBlanca2")
  (Rendering|Material|SetMaterial (Variables|/Script/TimerJamProyect.TimerJamProyectOffroadCar|GetChassis _asbp_offroad_car_pawn) 12 "/Game/Vehicles/OffroadCar/CarMaterials/LuzNaranja2.LuzNaranja2")
  (Rendering|Material|SetMaterial (Variables|/Script/TimerJamProyect.TimerJamProyectOffroadCar|GetChassis _asbp_offroad_car_pawn) 12 "/Game/Vehicles/OffroadCar/CarMaterials/LuzNaranja2.LuzNaranja2")
  ;[0.1198 0.04784 0] Maletin
  (Rendering|Material|SetMaterial (Variables|/Game/VehicleTemplate/Blueprints/OffroadCar/BP_OffroadCar_Pawn.BP_OffroadCar_Pawn_C|GetSuitcase _asbp_offroad_car_pawn) 0 "/Game/Vehicles/OffroadCar/Renault12/Mat_Case2.Mat_Case2")
  ;[0.05729 0.05729 0.05729] Ruedas
  (Rendering|Material|SetMaterial (Variables|/Script/TimerJamProyect.TimerJamProyectOffroadCar|GetTireFrontLeft _asbp_offroad_car_pawn) 0 "/Game/Vehicles/OffroadCar/CarMaterials/Plastico2.Plastico2")
  (Rendering|Material|SetMaterial (Variables|/Script/TimerJamProyect.TimerJamProyectOffroadCar|GetTireFrontLeft _asbp_offroad_car_pawn) 1 "/Game/Vehicles/OffroadCar/CarMaterials/Goma2.Goma2")
  ;[1 0.8826 0.3051] Parrilla
  (Rendering|Material|SetMaterial (Variables|/Game/VehicleTemplate/Blueprints/OffroadCar/BP_OffroadCar_Pawn.BP_OffroadCar_Pawn_C|Getparrila _asbp_offroad_car_pawn) 0 "/Game/Vehicles/OffroadCar/CarMaterials/Plastico2.Plastico2")
  (Rendering|Material|SetMaterial (Variables|/Game/VehicleTemplate/Blueprints/OffroadCar/BP_OffroadCar_Pawn.BP_OffroadCar_Pawn_C|Getparrila _asbp_offroad_car_pawn) 3 "/Game/Vehicles/OffroadCar/CarMaterials/Plastico2.Plastico2")
  (Rendering|Material|SetMaterial (Variables|/Game/VehicleTemplate/Blueprints/OffroadCar/BP_OffroadCar_Pawn.BP_OffroadCar_Pawn_C|Getparrila _asbp_offroad_car_pawn) 5 "/Game/Vehicles/OffroadCar/CarMaterials/Plastico2.Plastico2")
  (Rendering|Material|SetMaterial (Variables|/Game/VehicleTemplate/Blueprints/OffroadCar/BP_OffroadCar_Pawn.BP_OffroadCar_Pawn_C|Getparrila _asbp_offroad_car_pawn) 7 "/Game/Vehicles/OffroadCar/CarMaterials/Plastico2.Plastico2")
  (Rendering|Material|SetMaterial (Variables|/Game/VehicleTemplate/Blueprints/OffroadCar/BP_OffroadCar_Pawn.BP_OffroadCar_Pawn_C|Getparrila _asbp_offroad_car_pawn) 9 "/Game/Vehicles/OffroadCar/CarMaterials/Plastico2.Plastico2")
  ;[1 1 1] ParedInvisible
  (Development|SetHiddeninGame (Variables|Default|GetPared) false false)
  (Collision|SetCollisionEnabled (Variables|Default|GetPared) "QueryAndPhysics")
  (Utilities|FlowControl|Delay 5.0)
  (Development|SetHiddeninGame (Variables|Default|GetPared1) false false)
  (Collision|SetCollisionEnabled (Variables|Default|GetPared1) "QueryAndPhysics"))

(event OnComponentEndOverlap(BoxDetectora)
  (params (OverlappedComponent :type Primitive%20Component%20Object%20Reference) (OtherActor :type Actor%20Object%20Reference) (OtherComp :type Primitive%20Component%20Object%20Reference) (OtherBodyIndex :type Integer))
  ;[0.8298 0.3785 1] Sonido de cambio corto
  (Audio|PlaySound2D "/Game/Sounds/Efects/SonidoSpray.SonidoSpray" 1.0 1.0 0.0 0 0))

(fn ConstructionScript)